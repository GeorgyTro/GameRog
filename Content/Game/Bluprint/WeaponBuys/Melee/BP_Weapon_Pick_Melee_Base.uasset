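; Base Blueprint for a melee weapon pickup that the player can interact with while standing in its collision volume.
; Overlapping PickCollision binds the PickUp event to the player character's interact and shows its weapon HUD widget; leaving unbinds it and removes the widget.
; BeginPlay caches the player character reference.
; PickUp is empty here, and the DestroyActor logic is disconnected.
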(event OnComponentBeginOverlap(PickCollision)
  (params (OverlappedComponent :type Primitive%20Component%20Object%20Reference) (OtherActor :type Actor%20Object%20Reference) (OtherComp :type Primitive%20Component%20Object%20Reference) (OtherBodyIndex :type Integer) (bFromSweep :type Boolean) (SweepResult :type Hit%20Result%20Structure%20%28by%20ref%29))
  (bind _asplayer_character_game (Utilities|Casting|CastToPlayerCharacterGame OtherActor))
  (EventDispatchers|BindEventtoInteract _asplayer_character_game (delegate Custom|PickUp))
  (if (not (UserInterface|Viewport|IsinViewport (Variables|/Game/AdvancedLocomotionV4/Blueprints/CharacterLogic/PlayerCharacterGame.PlayerCharacterGame_C|GetWeapon%20Hud%20Ref _asplayer_character_game)))
    (UserInterface|Viewport|AddtoViewport (Variables|/Game/AdvancedLocomotionV4/Blueprints/CharacterLogic/PlayerCharacterGame.PlayerCharacterGame_C|GetWeapon%20Hud%20Ref _asplayer_character_game) 0)))

(event OnComponentEndOverlap(PickCollision)
  (params (OverlappedComponent :type Primitive%20Component%20Object%20Reference) (OtherActor :type Actor%20Object%20Reference) (OtherComp :type Primitive%20Component%20Object%20Reference) (OtherBodyIndex :type Integer))
  (bind _asplayer_character_game (Utilities|Casting|CastToPlayerCharacterGame OtherActor))
  (EventDispatchers|UnbindEventfromInteract _asplayer_character_game (delegate Custom|PickUp))
  (Widget|RemovefromParent (Variables|/Game/AdvancedLocomotionV4/Blueprints/CharacterLogic/PlayerCharacterGame.PlayerCharacterGame_C|GetWeapon%20Hud%20Ref _asplayer_character_game)))

(event Custom|PickUp)

(event EventBeginPlay
  ;[0 0.3906 1] BeginPlay
  (bind _asplayer_character_game (Utilities|Casting|CastToPlayerCharacterGame (Game|Player|GetPlayerPawn 0)))
  (Variables|Reference|Setplayer%20Ref _asplayer_character_game))

(fn ConstructionScript)