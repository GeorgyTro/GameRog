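; BP_LPSP_Target is a shooting-range target that reacts differently to point hits and explosions through damage interface events.
; A point hit on an active target plays the fall animation and sound, deactivates it, then raises and reactivates it after a random delay.
; An explosion spawns a BP_LPSP_Destroyed_Target at the mesh transform and destroys the actor.
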(event EventDamage
  (params (Damage :type Float%20%28single-precision%29) (DamageType :type DamageType%20Enum :default "NewEnumerator0") (BoneName :type Name :default "None") (ImpulseValue :type Vector :default "0, 0, 0") (HitLocation :type Vector :default "0, 0, 0"))
  (switch Utilities|FlowControl|Switch|SwitchonDamageType DamageType
    (:NewEnumerator0
      ;[1 0.03719 0] Point Damage
      (|CGraphDamagePoint))
    (:NewEnumerator1
      ;[1 0.1603 0] Radial Damage
      (Game|SpawnActorfromClass "/LPSPSample/LPSPSample/Useable/Damageables/BP_LPSP_Destroyed_Target.BP_LPSP_Destroyed_Target_C" (Transformation|GetWorldTransform (Variables|Default|GetMesh)) "AlwaysSpawn" 0 0)
      (Actor|DestroyActor))))

(event EventOnReceiveDamagePoint
  ;[1 0.03719 0] Point Damage
  (|CGraphDamagePoint))

(event EventOnReceiveDamageRadial
  ;[1 0.1603 0] Radial Damage
  (Game|SpawnActorfromClass "/LPSPSample/LPSPSample/Useable/Damageables/BP_LPSP_Destroyed_Target.BP_LPSP_Destroyed_Target_C" (Transformation|GetWorldTransform (Variables|Default|GetMesh)) "AlwaysSpawn" 0 0)
  (Actor|DestroyActor))

(fn ConstructionScript)