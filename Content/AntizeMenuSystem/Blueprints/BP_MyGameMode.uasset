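; Game mode for the Antize menu system that handles player joins, departures and an example difficulty setting.
; In multiplayer, a login triggers a delayed name refresh on every BP_MyCharacter through MultiSetName, and a logout prints a message.
; In single player, it restores the pawn to the saved transform from the game instance, raised slightly, retrying on a short delay until the pawn exists.
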(event Custom|ChangeDifficulty
  (params (NewDifficulty :type E_Difficulty%20Enum :default "NewEnumerator0"))
  ;[1 1 1] Difficulty changed (Exemple)
  (Variables|Default|SetCurrentDifficulty NewDifficulty))

(event EventOnLogout
  (params (ExitingController :type Controller%20Object%20Reference))
  ;[1 1 1] On player left server
  (bind _asbp_my_game_instance (Utilities|Casting|CastToBP_MyGameInstance (Game|GetGameInstance)))
  (if (Variables|/Game/AntizeMenuSystem/Blueprints/BP_MyGameInstance.BP_MyGameInstance_C|GetMultiplayer? _asbp_my_game_instance)
    (Development|PrintString "Player left" true true "(R=1.000000,G=0.944563,B=0.098612,A=1.000000)" 1e+01)))

(event EventPostLogin
  (params (NewPlayer :type Player%20Controller%20Object%20Reference))
  (bind _returnvalue (Pawn|GetControlledPawn NewPlayer))
  ;[1 1 1] On new player
  (bind _asbp_my_game_instance (Utilities|Casting|CastToBP_MyGameInstance (Game|GetGameInstance)))
  (if (Variables|/Game/AntizeMenuSystem/Blueprints/BP_MyGameInstance.BP_MyGameInstance_C|GetMultiplayer? _asbp_my_game_instance)
    ;;[1 1 1] In multiplayer call for refresh playername - SetName
    (Utilities|FlowControl|Delay 1.0)
    (bind _outactors (Actor|GetAllActorsOfClass "/Game/AntizeMenuSystem/Blueprints/BP_MyCharacter.BP_MyCharacter_C"))
    (for _array_element _outactors
      (Utilities|IsValid _array_element
        (:Is%20Valid
          (Default|MultiSetName _array_element))))
    (else
      ;;[1 1 1] Spawn player to last save point position (Add 100 for correction)
      (Utilities|IsValid (Variables|/Game/AntizeMenuSystem/Blueprints/BP_MyGameInstance.BP_MyGameInstance_C|GetMyGameSave _asbp_my_game_instance)
        (:Is%20Valid
          (if (Math|Vector|NotEqual(Vector) (.Location (Math|Transform|BreakTransform (Variables|/Game/AntizeMenuSystem/Blueprints/SaveGame/BP_MySaveGame.BP_MySaveGame_C|GetPlayerPosition (Variables|/Game/AntizeMenuSystem/Blueprints/BP_MyGameInstance.BP_MyGameInstance_C|GetMyGameSave _asbp_my_game_instance)))) "0, 0, 0" 0.0001)
            (Utilities|IsValid _returnvalue :!label _label
              (:Is%20Valid
                (Transformation|SetActorTransform _returnvalue (Math|Transform|MakeTransform (+ (.Location (Math|Transform|BreakTransform (Variables|/Game/AntizeMenuSystem/Blueprints/SaveGame/BP_MySaveGame.BP_MySaveGame_C|GetPlayerPosition (Variables|/Game/AntizeMenuSystem/Blueprints/BP_MyGameInstance.BP_MyGameInstance_C|GetMyGameSave _asbp_my_game_instance)))) "0,0.000000,100.000000") (.Rotation (Math|Transform|BreakTransform (Variables|/Game/AntizeMenuSystem/Blueprints/SaveGame/BP_MySaveGame.BP_MySaveGame_C|GetPlayerPosition (Variables|/Game/AntizeMenuSystem/Blueprints/BP_MyGameInstance.BP_MyGameInstance_C|GetMyGameSave _asbp_my_game_instance)))) (.Scale (Math|Transform|BreakTransform (Variables|/Game/AntizeMenuSystem/Blueprints/SaveGame/BP_MySaveGame.BP_MySaveGame_C|GetPlayerPosition (Variables|/Game/AntizeMenuSystem/Blueprints/BP_MyGameInstance.BP_MyGameInstance_C|GetMyGameSave _asbp_my_game_instance)))))))
              (:Is%20Not%20Valid
                (Utilities|FlowControl|Delay 0.01)
                (goto _label)))))))))

(fn ConstructionScript)