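; Template character Blueprint for AntizeMenuSystem, holding logic meant to be copied into a game's Character to connect it to the menu.
; On BeginPlay, the local player sends the GameInstance username to the server for replication in multiplayer, or hides the name widget otherwise.
; Interface events store mouse inversion and sensitivity from the options widget, and key requests forward to the controller.
; GetCanPass gates input by gamepad or keyboard/mouse mode, though the gamepad-key check is unwired.
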(event Custom|Server_SetName
  (params (InText :type Text%20%28by%20ref%29))
  ;[0 0.9062 1] Add this and Interfaces MSG_RequestKey to your Character
  ;;[0 0.8359 1] Set username (Replicated)
  (Networking|SwitchHasAuthority
    (:Authority
      (Variables|InGame|SetUsername InText))))

(event Custom|SetName
  ;[0 0.9062 1] Add this and Interfaces MSG_RequestKey to your Character
  ;;[0 0.8359 1] Set username (Replicated)
  (bind _asbp_my_game_instance (Utilities|Casting|CastToBP_MyGameInstance (Game|GetGameInstance)))
  (if (Variables|/Game/AntizeMenuSystem/Blueprints/BP_MyGameInstance.BP_MyGameInstance_C|GetMultiplayer? _asbp_my_game_instance)
    (CallFunction|ServerSetName (Variables|/Game/AntizeMenuSystem/Blueprints/BP_MyGameInstance.BP_MyGameInstance_C|GetUsername _asbp_my_game_instance))
    (else
      (Rendering|SetVisibility (Variables|Default|GetWidget) false false))))

(event EventMSGChangeInvertMouse
  (params (InvertMouse :type Boolean))
  ;[0 0.9062 1] Add this and Interfaces MSG_RequestKey to your Character
  ;;[1 0.1875 0.1875] Change mouse setting from "W_Options" (Set 1 to default value sensitivity)
  ;;;[0 0.9427 0.2694] Be sure to add "AntizeInterface" in character | Class Settings -> in "Interfaces" category click on "Add" -> BP_AntizeInterface -> Compile -> Copy Past
  (Variables|Inputs|SetInvertMouse? InvertMouse))

(event EventMSGChangeSensitivity
  (params (Sensitivity :type Float%20%28single-precision%29))
  ;[0 0.9062 1] Add this and Interfaces MSG_RequestKey to your Character
  ;;[1 0.1875 0.1875] Change mouse setting from "W_Options" (Set 1 to default value sensitivity)
  ;;;[0 0.9427 0.2694] Be sure to add "AntizeInterface" in character | Class Settings -> in "Interfaces" category click on "Add" -> BP_AntizeInterface -> Compile -> Copy Past
  (Variables|Inputs|SetSensitivity Sensitivity))

(event EventBeginPlay
  ;[0 0.9062 1] Add this and Interfaces MSG_RequestKey to your Character
  ;;[0 0.9427 0.2694] Get Interact Key (Delay for option load)
  (if (Pawn|IsLocallyControlled)
    (CallFunction|SetName)))

(fn ConstructionScript)

(fn GetCanPass
  (return (Utilities|Select :Index (Variables|Inputs|Block|GetMyInputMode) :NewEnumerator0 true :NewEnumerator1 (not (Variables|Inputs|Block|GetIsGamepadKey?)) :NewEnumerator2 (Variables|Inputs|Block|GetIsGamepadKey?))))

(fn MSGIsKeyEditing
  (return false))

(fn MSGRequestKey
  (params (Action? :type Boolean) (ActionName :type E_TemplateControlAction%20Enum :default "NewEnumerator0") (AxisName :type E_TemplateControlAxis%20Enum :default "NewEnumerator0"))
  (bind _returnvalue (Pawn|GetController))
  (Utilities|IsValid _returnvalue
    (:Is%20Valid
      (bind _mykey (Class|BPAntizeInterface|MSGRequestKey(Message) _returnvalue Action? ActionName AxisName))
      (return _mykey))
    (:Is%20Not%20Valid
      (return ""))))